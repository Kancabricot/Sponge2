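; BP_BubbleJump is a bubble projectile that knocks a BP_SpongePlayer away when it touches them, then pops.
; On spawn, a timeline eases its forward projectile speed down and pops it when finished, while hit collision enables after a short delay.
; On overlap, it aims a helper component toward the player and launches them that way, scaled by BubbleForce.
; Any overlap pops it, spawning an effect and destroying the actor.
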(event OnComponentBeginOverlap(HitCollision)
  (params (OverlappedComponent :type Primitive%20Component%20Object%20Reference) (OtherActor :type Actor%20Object%20Reference) (OtherComp :type Primitive%20Component%20Object%20Reference) (OtherBodyIndex :type Integer) (bFromSweep :type Boolean) (SweepResult :type Hit%20Result%20Structure%20%28by%20ref%29))
  (bind _asbp_sponge_player (Utilities|Casting|CastToBP_SpongePlayer OtherActor)
    (:then
      (CallFunction|ForwardforLaunch _asbp_sponge_player)
      (Character|LaunchCharacter _asbp_sponge_player (* (Math|Vector|GetForwardVector (Variables|Default|GetLaunchRotation)) (Variables|/Game/05-Blueprints/PDA_Iteration.PDA_Iteration_C|GetBubbleForce (Variables|Default|GetIteration))) false false))
    (:CastFailed
      _))
  (CallFunction|BubbleDeath))

(event EventBeginPlay
  (Utilities|FlowControl|Sequence
    (:then_0
      (bind _movementtrack (Timeline|BubbleMove PlayFromStart)
        (:Update
          (Variables|/Script/Engine.MovementComponent|SetVelocity (Variables|Default|GetProjectileMovement) (* (Transformation|GetActorForwardVector) (Math|Float|Lerp 1e+03 1e+02 _movementtrack))))
        (:Finished
          (CallFunction|BubbleDeath))))
    (:then_1
      (Utilities|FlowControl|Delay 0.2)
      (Collision|SetCollisionEnabled (Variables|Default|GetHitCollision) "QueryAndPhysics"))))

(fn ConstructionScript)

(fn ForwardforLaunch
  (params (Target :type Actor%20Object%20Reference))
  (Transformation|SetWorldRotation (Variables|Default|GetLaunchRotation) (Math|Rotator|FindLookatRotation (Transformation|GetActorLocation) (Transformation|GetActorLocation Target)) false false))

(fn BubbleDeath
  (Niagara|SpawnSystematLocation "/Game/04-VFX/01-NiagaraSystem/NS_BubbleTest.NS_BubbleTest" (Transformation|GetWorldLocation (Variables|Default|GetSM_Bubble)))
  (Actor|DestroyActor))