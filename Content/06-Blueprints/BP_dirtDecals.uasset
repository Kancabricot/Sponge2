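; Dirt decal actor that wears away as it takes bubble damage.
; Each BubbleDamage call decrements Life and shrinks the Decal's world scale on Y and Z, leaving X unchanged.
; Once Life reaches zero or below, it hands off to the parent class's BubbleDamage.
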(fn ConstructionScript
  (|CallParentFunction))

(fn BubbleDamage
  (Variables|Default|SetLife (- (Variables|Default|GetLife) 1))
  (Transformation|SetWorldScale3D (Variables|Default|GetDecal) (- (Transformation|GetWorldScale (Variables|Default|GetDecal)) "0.000000,0.200000,0.200000"))
  (if (<= (Variables|Default|GetLife) 0)
    (|CallParentFunction)))