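; Base NPC that travels along a spline, periodically leaves dirt decals and can be destroyed by bubble shots.
; When FollowSpline is set, a timeline drives its transform along the referenced spline.
; A random timer pauses movement for a montage (or short delay), then spawns optional Niagara VFX and a decal before resuming.
; BP_BubbleShoot overlaps briefly flash an overlay on the skeletal or static mesh and decrement PV, destroying the actor at zero.
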(event OnComponentBeginOverlap(Box)
  (params (OverlappedComponent :type Primitive%20Component%20Object%20Reference) (OtherActor :type Actor%20Object%20Reference) (OtherComp :type Primitive%20Component%20Object%20Reference) (OtherBodyIndex :type Integer) (bFromSweep :type Boolean) (SweepResult :type Hit%20Result%20Structure%20%28by%20ref%29))
  (Utilities|Casting|CastToBP_BubbleShoot OtherActor)
  (Utilities|FlowControl|DoOnce false :!label _label
    (:Completed
      (CallFunction|SetOverlayMaterial)
      (bind _output_get (Variables|Default|SetPV (- (Variables|Default|GetPV) 1.0)))
      (if (<= _output_get 0.0)
        (Actor|DestroyActor)
        (goto _label Reset)
        (else
          (goto _label Reset))))))

(event Custom|Move%20Along%20Spline
  (bind _spline (Variables|Default|GetSpline))
  (bind _spline_2 (Variables|/Game/06-Blueprints/NPC/BP_NPC_Spline.BP_NPC_Spline_C|GetSpline _spline))
  (Variables|Default|GetSpline
    (:then
      (bind _alpha (Timeline|Timeline_MoveObject Play)
        (:Update
          (Transformation|SetActorTransform self (Math|Transform|MakeTransform (Spline|GetLocationatDistanceAlongSpline _spline_2 (Math|Float|Lerp 0.0 (Spline|GetSplineLength (Variables|/Game/06-Blueprints/NPC/BP_NPC_Spline.BP_NPC_Spline_C|GetSpline (Variables|Default|GetSpline))) _alpha) "World") (Spline|GetRotationatDistanceAlongSpline _spline_2 (Math|Float|Lerp 0.0 (Spline|GetSplineLength (Variables|/Game/06-Blueprints/NPC/BP_NPC_Spline.BP_NPC_Spline_C|GetSpline (Variables|Default|GetSpline))) _alpha) "World") "1.000000,1.000000,1.000000")))))
    (:else
      (Development|PrintString "No spline ref" true true "(R=1.000000,G=0.000000,B=0.000000,A=1.000000)"))))

(event Custom|Stop%20Move%20Along%20Spline
  (bind _spline (Variables|Default|GetSpline))
  (bind _spline_2 (Variables|/Game/06-Blueprints/NPC/BP_NPC_Spline.BP_NPC_Spline_C|GetSpline _spline))
  (bind _alpha (Timeline|Timeline_MoveObject Stop)
    (:Update
      (Transformation|SetActorTransform self (Math|Transform|MakeTransform (Spline|GetLocationatDistanceAlongSpline _spline_2 (Math|Float|Lerp 0.0 (Spline|GetSplineLength (Variables|/Game/06-Blueprints/NPC/BP_NPC_Spline.BP_NPC_Spline_C|GetSpline (Variables|Default|GetSpline))) _alpha) "World") (Spline|GetRotationatDistanceAlongSpline _spline_2 (Math|Float|Lerp 0.0 (Spline|GetSplineLength (Variables|/Game/06-Blueprints/NPC/BP_NPC_Spline.BP_NPC_Spline_C|GetSpline (Variables|Default|GetSpline))) _alpha) "World") "1.000000,1.000000,1.000000")))))

(event Custom|Play%20Animation
  (CallFunction|StopMoveAlongSpline)
  (if (Variables|Default|GetHave%20Skeletal%20Mesh)
    (Animation|Montage|PlayMontage (Variables|Default|GetSkeletalMesh) (Variables|Default|GetMontage%20to%20Play)
      (:OnCompleted
        _)
      (:OnInterrupted
        _))
    (else
      (Utilities|FlowControl|Delay 1.0)))
  (CallFunction|CreateDecal))

(event Custom|Create%20Decal
  (bind _niagara_system (Variables|Default|GetNiagara%20System)
    (:then
      (Niagara|SpawnSystematLocation _niagara_system (Transformation|GetWorldLocation (Variables|Default|GetVfx%20Spawn%20Location)))
      (Utilities|FlowControl|Delay 1.0))
    (:else
      _))
  (bind _returnvalue (Game|SpawnActorfromClass "/Game/06-Blueprints/BP_dirtDecals.BP_dirtDecals_C" (Math|Transform|MakeTransform (Transformation|GetWorldLocation (Variables|Default|GetDecal%20Spawn%20Location)) "-90.000000,0.000000,0.000000" "1.000000,1.000000,1.000000") "Undefined" "MultiplyWithRoot" 0 0))
  (Rendering|Components|Decal|SetDecalMaterial (Variables|/Game/06-Blueprints/BP_dirtDecals.BP_dirtDecals_C|GetDecal _returnvalue) (Utilities|Array|Get(acopy) (Variables|Default|GetDecal%20Materials) (select (Variables|Default|GetRandom%20Decal) (Math|Random|RandomIntegerinRange 0 (- (Utilities|Array|Length (Variables|Default|GetDecal%20Materials)) 1)) 0)))
  (CallFunction|MoveAlongSpline)
  (Utilities|Time|ClearandInvalidateTimerbyHandle (Variables|Default|GetTimer%20Handler))
  (CallFunction|StartTimer))

(event Custom|Start%20Timer
  (bind _returnvalue (Utilities|Time|SetTimerbyEvent (delegate Custom|Play%20Animation) (Math|Random|RandomFloatinRange 15.0 3e+01)))
  (Variables|Default|SetTimer%20Handler _returnvalue))

(event Custom|Set%20Overlay%20Material
  (if (Variables|Default|GetHave%20Skeletal%20Mesh)
    (Rendering|Material|SetOverlayMaterial (Variables|Default|GetSkeletalMesh) (Variables|Default|GetOverlay%20Material) :!class /Script/Engine.MeshComponent)
    (Utilities|FlowControl|Delay 0.5)
    (Rendering|Material|SetOverlayMaterial (Variables|Default|GetSkeletalMesh) 0 :!class /Script/Engine.MeshComponent)
    (else
      (Rendering|Material|SetOverlayMaterial (Variables|Default|GetStaticMesh) (Variables|Default|GetOverlay%20Material) :!class /Script/Engine.MeshComponent)
      (Utilities|FlowControl|Delay 0.5)
      (Rendering|Material|SetOverlayMaterial (Variables|Default|GetStaticMesh) 0 :!class /Script/Engine.MeshComponent))))

(event EventBeginPlay
  (if (Variables|Default|GetFollow%20Spline)
    (Components|Timeline|SetPlayRate (Variables|Default|GetTimeline_MoveObject) (Variables|Default|GetPlay%20Rate))
    (CallFunction|MoveAlongSpline)
    (CallFunction|StartTimer)))

(fn ConstructionScript)