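; BP_dirt is a dirt object that registers itself with the game mode and is destroyed by bubble damage.
; On BeginPlay it casts and stores the BP_ThirdPersonGameMode reference, then calls AddIndex with its BIsTuto flag, which appears to mark tutorial dirt.
; BubbleDamage calls RemoveIndex with the same flag and destroys the actor, so the game mode can track the remaining dirt.
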(event EventBeginPlay
  (bind _asbp_third_person_game_mode (Utilities|Casting|CastToBP_ThirdPersonGameMode (Game|GetGameMode)))
  (bind _output_get (Variables|Default|SetGameModeRef _asbp_third_person_game_mode))
  (CallFunction|GetGameModeRef _output_get))

(fn ConstructionScript)

(fn BubbleDamage
  (Default|RemoveIndex (Variables|Default|GetGameModeRef) (Variables|Default|Getb_IsTuto))
  (Actor|DestroyActor))

(fn GetGameModeRef
  (params (GameModeRef :type BP%20Third%20Person%20Game%20Mode%20Object%20Reference))
  (bind _output_get (Variables|Default|SetGameModeRef GameModeRef))
  (Default|AddIndex _output_get (Variables|Default|Getb_IsTuto)))