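; BP_ControllerMenu handles Enhanced Input for menu navigation.
; Up and down inputs pass -1 or 1 to ControllerMovement on UIMenuRef, while accept only prints a debug string.
; The setup that shows the cursor, creates WG_Menu, stores it in UIMenuRef and adds IMC_Menu is disconnected and never runs, so nothing in this Blueprint assigns that reference.
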(event Input|EnhancedActionEvents|EnhancedInputActionIA_MenuUp
  (params (ActionValue :type Boolean) (ElapsedSeconds :type Float%20%28double-precision%29) (TriggeredSeconds :type Float%20%28double-precision%29) (InputAction :type Input%20Action%20Object%20Reference :default "/Game/Input/Actions/IA_MenuUp.IA_MenuUp"))
  (:Started
    (Development|PrintString "Up" true true "(R=1.000000,G=0.000000,B=0.000000,A=1.000000)")
    (Default|ControllerMovement (Variables|Default|GetUIMenuRef) -1)))

(event Input|EnhancedActionEvents|EnhancedInputActionIA_MenuDown
  (params (ActionValue :type Boolean) (ElapsedSeconds :type Float%20%28double-precision%29) (TriggeredSeconds :type Float%20%28double-precision%29) (InputAction :type Input%20Action%20Object%20Reference :default "/Game/Input/Actions/IA_MenuDown.IA_MenuDown"))
  (:Started
    (Development|PrintString "Down" true true "(R=1.000000,G=0.000000,B=0.000000,A=1.000000)")
    (Default|ControllerMovement (Variables|Default|GetUIMenuRef) 1)))

(event Input|EnhancedActionEvents|EnhancedInputActionIA_MenuAccept
  (params (ActionValue :type Boolean) (ElapsedSeconds :type Float%20%28double-precision%29) (TriggeredSeconds :type Float%20%28double-precision%29) (InputAction :type Input%20Action%20Object%20Reference :default "/Game/Input/Actions/IA_MenuAccept.IA_MenuAccept"))
  (:Started
    (Development|PrintString "Accept" true true "(R=1.000000,G=0.000000,B=0.000000,A=1.000000)")))

(event EventBeginPlay)

(fn ConstructionScript)