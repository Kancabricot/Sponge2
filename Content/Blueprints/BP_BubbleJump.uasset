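; BP_BubbleJump is a bubble projectile that knocks a BP_SpongePlayer away when it touches one.
; On BeginPlay a timeline eases its forward velocity from fast to slow.
; On overlap it aims the LaunchRotation component from the bubble toward the player and launches the character along that direction, adding to existing velocity.
; The bubble destroys itself on any overlap, whether or not it hit a player.
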(event OnComponentBeginOverlap(HitCollision)
  (params (OverlappedComponent :type Primitive%20Component%20Object%20Reference) (OtherActor :type Actor%20Object%20Reference) (OtherComp :type Primitive%20Component%20Object%20Reference) (OtherBodyIndex :type Integer) (bFromSweep :type Boolean) (SweepResult :type Hit%20Result%20Structure%20%28by%20ref%29))
  (bind _asbp_sponge_player (Utilities|Casting|CastToBP_SpongePlayer OtherActor)
    (:then
      (CallFunction|ForwardforLaunch _asbp_sponge_player)
      (Character|LaunchCharacter _asbp_sponge_player (* (Math|Vector|GetForwardVector (Variables|Default|GetLaunchRotation)) 1500) false false))
    (:CastFailed
      _))
  (Actor|DestroyActor))

(event EventBeginPlay
  (bind _movementtrack (Timeline|BubbleMove PlayFromStart)
    (:Update
      (Variables|/Script/Engine.MovementComponent|SetVelocity (Variables|Default|GetProjectileMovement) (* (Transformation|GetActorForwardVector) (Math|Float|Lerp 1e+03 1e+02 _movementtrack))))))

(fn ConstructionScript)

(fn ForwardforLaunch
  (params (Target :type Actor%20Object%20Reference))
  (Transformation|SetWorldRotation (Variables|Default|GetLaunchRotation) (Math|Rotator|FindLookatRotation (Transformation|GetActorLocation) (Transformation|GetActorLocation Target)) false false))